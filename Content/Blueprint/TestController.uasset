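; Test player controller that exercises the inventory component and its UI panel.
; The construction script registers a weapon list type with the Inventory component.
; On BeginPlay it creates a PanelBP widget, adds it to the viewport and hands it the Inventory.
; It then adds a stack of Weapon to the inventory and has the panel query for Weapon.
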(event `self.ReceiveBeginPlay`
  (bind _returnvalue (`|CreateWidget` "/Game/Blueprint/InventorySystem/PanelBP.PanelBP_C" self))
  (`UserWidget.AddToViewport` _returnvalue 0)
  (`InventoryPanel.SetInventoryComponent` _returnvalue (`self.Inventory`))
  (`InventoryComponent.AddToInventory` (`self.Inventory`) "/Game/Blueprint/InventorySystem/Object/Weapon/Weapon.Weapon_C" 7)
  (`InventoryPanel.QueryFor` _returnvalue "/Game/Blueprint/InventorySystem/Object/Weapon/Weapon.Weapon_C"))

(fn `UserConstructionScript`
  (`InventoryComponent.AddInventoryListType` (`self.Inventory`) "/Game/Blueprint/InventorySystem/Object/Weapon/WeaponList.WeaponList_C"))