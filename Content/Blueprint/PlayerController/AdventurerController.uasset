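; AdventurerController is a player controller that owns the player's inventory component and its on-screen window.
; The construction script registers item, tool, weapon and armor lists, then seeds them with hardcoded weapons and potions and resizes the weapon list.
; BeginPlay creates the InventoryWindow widget and hands it the component.
; The Test input toggles that window in the viewport, switching between game-only and game-and-UI input modes.
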(event `self.ReceiveBeginPlay`
  (bind _returnvalue (`|CreateWidget` "/Game/Blueprint/Inventory/UI/InventoryWindow.InventoryWindow_C" self))
  (bind _output_get (set `self.InventoryWindow` _returnvalue))
  (`/Game/Blueprint/Inventory/UI/InventoryWindow.SetInventoryComponent` _output_get (`self.InventoryComponent`)))

(event `InputAction|Test`
  (params (Key :type "Key Structure"))
  (bind _inventorywindow (`self.InventoryWindow`))
  (:`Pressed`
    (if (`Widget.IsInViewport` (`self.InventoryWindow`))
      (`Widget.RemoveFromParent` _inventorywindow)
      (`WidgetBlueprintLibrary.SetInputMode_GameOnly` self)
      (else
        (`UserWidget.AddToViewport` _inventorywindow 0)
        (`WidgetBlueprintLibrary.SetInputMode_GameAndUIEx` self _inventorywindow)))))

(fn `FillInventory`
  (bind _inventorycomponent (`self.InventoryComponent`))
  (`InventoryComponent.AddBySubclass` _inventorycomponent "/Game/Blueprint/Inventory/Equipment/Weapons/Sword.Sword_C" 4)
  (`InventoryComponent.AddBySubclass` _inventorycomponent "/Game/Blueprint/Inventory/Equipment/Weapons/WarScythe.WarScythe_C" 6)
  (bind _returnvalue (`InventoryComponent.GetInventoryListFor` (`self.InventoryComponent`) "/Game/Blueprint/Inventory/Equipment/Base/Weapon.Weapon_C"))
  (`InventoryList.MofifyListSize` _returnvalue 17)
  (`InventoryComponent.AddBySubclass` _inventorycomponent "/Game/Blueprint/Inventory/Consumable/Item/XPotion.XPotion_C" 6))

(fn `InitializeInventoryComponent`
  (bind _inventorycomponent (`self.InventoryComponent`))
  (`InventoryComponent.AddInventoryListType` _inventorycomponent "/Game/Blueprint/Inventory/Lists/ItemList.ItemList_C")
  (`InventoryComponent.AddInventoryListType` _inventorycomponent "/Game/Blueprint/Inventory/Lists/ToolList.ToolList_C")
  (`InventoryComponent.AddInventoryListType` _inventorycomponent "/Game/Blueprint/Inventory/Lists/WeaponList.WeaponList_C")
  (`InventoryComponent.AddInventoryListType` _inventorycomponent "/Game/Blueprint/Inventory/Lists/ArmorList.ArmorList_C"))

(fn `UserConstructionScript`
  (`self.InitializeInventoryComponent`)
  (`self.FillInventory`))